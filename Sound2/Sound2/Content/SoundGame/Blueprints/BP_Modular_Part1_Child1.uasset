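; BP_Modular_Part1_Child1 is a child modular part Blueprint with a door that swings automatically on proximity.
; Overlapping the Sphere component plays the DoorAnimation timeline, and ending the overlap reverses it.
; The timeline's Door track drives a yaw lerp on SMDoor's relative rotation across a quarter turn, with no filter on the overlapping actor.
; Construction defers to the parent.
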(event `self.Sphere.OnComponentBeginOverlap`
  (params (OverlappedComponent :type "PrimitiveComponent Object Reference") (OtherActor :type "Actor Object Reference") (OtherComp :type "PrimitiveComponent Object Reference") (OtherBodyIndex :type Integer) (bFromSweep :type Boolean) (SweepResult :type "HitResult Structure (by ref)"))
  (bind (_direction _door) (`Timeline|DoorAnimation` :!label _label)
    (:`Update`
      (`SceneComponent.K2_SetRelativeRotation` (`self.SM_Door`) (`KismetMathLibrary.MakeRotator` 0.0 0.0 (`KismetMathLibrary.Lerp` 90.0 0.0 _door)) false false))))

(event `self.Sphere.OnComponentEndOverlap`
  (params (OverlappedComponent :type "PrimitiveComponent Object Reference") (OtherActor :type "Actor Object Reference") (OtherComp :type "PrimitiveComponent Object Reference") (OtherBodyIndex :type Integer))
  (goto _label :!via `Reverse`))

(fn `UserConstructionScript`
  (`parent.UserConstructionScript`))