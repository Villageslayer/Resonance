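; BP_SoundBall is a bouncing ball actor that plays a test sound on spawn and on bounces, and destroys itself on the fourth bounce.
; Each hit rotates it from its velocity and repeats a persistent-debug line trace along that velocity, while a short retriggerable delay debounces bounce counting.
; The trace reads the surface type, but the SBall parameter is set to a zero BlockType, with no per-surface cases shown.
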(event `self.ReceiveBeginPlay`
  ;[0.15 0 0 0.5] Line Trace
  (`self.SetActorScale3D` (0.6 0.6 0.6))
  (`GameplayStatics.PlaySoundAtLocation` "/Game/SoundGame/Sounds/TestSound.TestSound" (`SceneComponent.K2_GetComponentLocation` (`self.Sphere`)) (struct) 1.0 1.0 0.0 null null null null)
  (`self.LineTraceSoundBlock`))

(event `self.ReceiveHit`
  (params (MyComp :type "PrimitiveComponent Object Reference") (Other :type "Actor Object Reference") (OtherComp :type "PrimitiveComponent Object Reference") (bSelfMoved :type Boolean) (HitLocation :type "Vector Structure") (HitNormal :type "Vector Structure") (NormalImpulse :type "Vector Structure") (Hit :type "HitResult Structure (by ref)"))
  ;[0.15 0 0 0.5] New Line Trace after Bounce // Destroy on 4th Bounce // Play Sound on Bounce
  (`|ExecutionSequence`
    (:`then_0`
      (`self.K2_SetActorRotation` (* (`KismetMathLibrary.Conv_VectorToRotator` (`self.GetVelocity`)) -1.0))
      (`self.LineTraceSoundBlock`))
    (:`then_1`
      (`KismetSystemLibrary.RetriggerableDelay` 0.01)
      (bind _result (`/Engine/EditorBlueprintResources/StandardMacros.IncrementInt` (`self.Bounces`))
        (:`  `
          (if (>= _result 4)
            (`self.K2_DestroyActor`)
            (else
              (`GameplayStatics.PlaySoundAtLocation` "/Game/SoundGame/Sounds/TestSound.TestSound" (`SceneComponent.K2_GetComponentLocation` (`self.Sphere`)) (struct) 1.0 1.0 0.0 null null null null))))))))

(fn `LineTraceSoundBlock`
  (bind _returnvalue (`SceneComponent.K2_GetComponentLocation` (`self.Sphere`)))
  (bind _outhit (`KismetSystemLibrary.LineTraceSingle` :`Start` _returnvalue :`End` (+ _returnvalue (`self.GetVelocity`)) :`TraceChannel` "TraceTypeQuery1" :`DrawDebugType` "Persistent"))
  (switch `EPhysicalSurface` (`GameplayStatics.GetSurfaceType` _outhit)
    (:`SurfaceType_Default`
      (set `self.BlockType` 0.0)
      (`FMODAudioComponent.SetParameter` (`self.SBall`) "SBall" (`self.BlockType`)))))

(fn `UserConstructionScript`)